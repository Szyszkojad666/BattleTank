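; Base tank pawn with a physics-simulated hull, shared by player and non-player control.
; Forward and turn inputs go to TankMovementComp, while aim inputs rotate the Gimbal in yaw and the SpringArm in pitch.
; The construction script snaps turret, barrel and both tracks onto mesh sockets and gives the body a heavy mass override.
; BeginPlay hides the health bar widget for player controllers, otherwise it sets the tank as the bar's owner.
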(event `InputAxis|MoveForward`
  (params (AxisValue :type "Float (single-precision)"))
  (`TankMovementComponent.MoveForward` (`self.TankMovementComp`) AxisValue))

(event `InputAxis|TurnRight`
  (params (AxisValue :type "Float (single-precision)"))
  (`TankMovementComponent.TurnRight` (`self.TankMovementComp`) AxisValue))

(event `InputAxis|AimPitch`
  (params (AxisValue :type "Float (single-precision)"))
  (`SceneComponent.K2_AddLocalRotation` (`self.SpringArm`) (`KismetMathLibrary.MakeRotator` 0.0 AxisValue) false false))

(event `InputAxis|AimYaw`
  (params (AxisValue :type "Float (single-precision)"))
  (`SceneComponent.K2_AddLocalRotation` (`self.Gimbal`) (`KismetMathLibrary.MakeRotator` 0.0 0.0 AxisValue) false false))

(event `self.ReceiveBeginPlay`
  (if (`Controller.IsPlayerController` (`self.GetController`))
    (`SceneComponent.SetVisibility` (`self.Widget`) false false)
    (else
      (bind _aswbp_healthbar (cast `/Game/UI/Widgets/WBP_Healthbar` (`WidgetComponent.GetUserWidgetObject` (`self.Widget`))))
      (set `/Game/UI/Widgets/WBP_Healthbar.OwnerPawn` self _aswbp_healthbar))))

(fn `UserConstructionScript`
  (bind _sm_body (`self.SM_Body`))
  (`SceneComponent.K2_AttachToComponent` (`self.TurretComp`) (`self.SM_Body`) "S_Turret" "SnapToTarget" "KeepRelative" "KeepRelative" true)
  (`SceneComponent.K2_AttachToComponent` (`self.Barrel`) (`self.TurretComp`) "S_Barrel" "SnapToTarget" "SnapToTarget" "KeepRelative" true)
  (`SceneComponent.K2_AttachToComponent` (`self.TrackL`) (`self.SM_Body`) "S_Track_L" "SnapToTarget" "SnapToTarget" "KeepRelative" true)
  (`SceneComponent.K2_AttachToComponent` (`self.TrackR`) (`self.SM_Body`) "S_Track_R" "SnapToTarget" "SnapToTarget" "KeepRelative" true)
  (`PrimitiveComponent.SetSimulatePhysics` _sm_body true)
  (`PrimitiveComponent.SetMassOverrideInKg` _sm_body "None" 40000.0 true))