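; Base Blueprint for a mortar unit, built from a body, turret and barrel and aimed through a TankAiming component.
; The construction script snaps the turret to the body's dome socket and the barrel to the turret's barrel socket, keeping relative scale.
; On BeginPlay it passes the barrel and turret references to the aiming component, reusing tank-named parts; Tick and overlap events are unused.
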(event `self.ReceiveBeginPlay`
  (`TankAimingComponent.Initialize` (`self.TankAiming`) (`self.TankBarrel`) (`self.TankTurret`)))

(fn `UserConstructionScript`
  (`SceneComponent.K2_AttachToComponent` (`self.TankTurret`) (`self.Body`) "S_Dome" "SnapToTarget" "SnapToTarget" "KeepRelative" true)
  (`SceneComponent.K2_AttachToComponent` (`self.TankBarrel`) (`self.TankTurret`) "S_Barrel" "SnapToTarget" "SnapToTarget" "KeepRelative" true))